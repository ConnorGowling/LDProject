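; Base actor for placeable interactables, dispatching Interact by type to pickup, note, web or switch behaviour.
; HighLight shows a sprite and overlay material, then a timer clears them if the player is far away; focus swaps to a type-based icon.
; Notes freeze and zoom the player and reuse the GameMode's widget; web opens through the GameMode in UI-only input.
; Pickup and switch responses are empty hooks, presumably for child Blueprints.
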(event `/Game/Blueprints/Placeables/interactions/Interact_BI.HighLight`
  (`SceneComponent.SetHiddenInGame` (`self. Highlight`) false false)
  (bind _returnvalue (`KismetSystemLibrary.K2_SetTimer` null "endhighlight" 0.3))
  (set `self.EndHighlightTimer` _returnvalue)
  (`MeshComponent.SetOverlayMaterial` (`self. Mesh`) "/Game/AdvancedLocomotionV4/CharacterAssets/MannequinSkeleton/Materials/OverlayTakeDown.OverlayTakeDown" false 0))

(event `/Game/Blueprints/Placeables/interactions/Interact_BI.Leave`
  (`SceneComponent.SetHiddenInGame` (`self. Highlight`) true false)
  (`BillboardComponent.SetSprite` (`self. Highlight`) "/Game/Blueprints/Placeables/interactions/Textures/mag_Glass.mag_Glass")
  (`MeshComponent.SetOverlayMaterial` (`self. Mesh`) null false 0))

(event `/Game/Blueprints/Placeables/interactions/Interact_BI.focused`
  (`BillboardComponent.SetSprite` (`self. Highlight`) (`self.focused sprite`)))

(event `/Game/Blueprints/Placeables/interactions/Interact_BI.Interact`
  (bind _returnvalue (`GameplayStatics.GetPlayerController` 0))
  (switch `/Game/AdvancedLocomotionV4/Blueprints/CharacterLogic/InteractType` (`self.interactType`)
    (:`NewEnumerator1`
      ;[1 1 1] start the interaction
      (`self.Pickup`))
    (:`NewEnumerator2`
      (`/Engine/EditorBlueprintResources/StandardMacros.DoOnce` false :!label _label
        (:`Completed`
          (bind _asals_anim_man_character_bp (cast `/Game/AdvancedLocomotionV4/Blueprints/CharacterLogic/ALS_AnimMan_CharacterBP` (`GameplayStatics.GetPlayerCharacter` 0)))
          (`CharacterMovementComponent.SetMovementMode` (`Character.CharacterMovement` _asals_anim_man_character_bp) "MOVE_None" 0)
          (`/Game/AdvancedLocomotionV4/Blueprints/CharacterLogic/ALS_AnimMan_CharacterBP.interactingCAmZoom` _asals_anim_man_character_bp)
          (bind _asals_game_mode_sp (cast `/Game/AdvancedLocomotionV4/Blueprints/GameModes/ALS_GameMode_SP` (`GameplayStatics.GetGameMode`)))
          (`self.CreateNote` _asals_game_mode_sp))))
    (:`NewEnumerator4`
      (bind _asals_game_mode_sp_2 (cast `/Game/AdvancedLocomotionV4/Blueprints/GameModes/ALS_GameMode_SP` (`GameplayStatics.GetGameMode`)))
      (`/Game/AdvancedLocomotionV4/Blueprints/GameModes/ALS_GameMode_SP.OpenWeb` _asals_game_mode_sp_2 (`self.WebAdress`))
      (set `PlayerController.bShowMouseCursor` true _returnvalue)
      (`WidgetBlueprintLibrary.SetInputMode_UIOnlyEx` _returnvalue null)
      (`CharacterMovementComponent.SetMovementMode` (`Character.CharacterMovement` (`GameplayStatics.GetPlayerCharacter` 0)) "MOVE_None" 0))
    (:`NewEnumerator5`
      (`self.RemoteInteractResponse`))))

(event `CloseNote`
  ;[1 1 1] start the interaction
  (goto _label :!via `Reset`))

(event `Pickup`)

(event `RemoteInteractResponse`)

(fn `CreateNote`
  (params (self2 :type "/Game/AdvancedLocomotionV4/Blueprints/GameModes/ALS_GameMode_SP Object Reference"))
  (bind _note (`/Game/AdvancedLocomotionV4/Blueprints/GameModes/ALS_GameMode_SP.Note` self2))
  (`/Engine/EditorBlueprintResources/StandardMacros.IsValid` _note
    (:`Is Valid`
      (`/Game/Blueprints/Placeables/interactions/wbp_Note_Widget.Initialise` _note (`self.Header`) (`self.Main Body Text`))
      (`UserWidget.AddToViewport` _note 0))
    (:`Is Not Valid`
      (bind _returnvalue (`|CreateWidget` "/Game/Blueprints/Placeables/interactions/wbp_Note_Widget.wbp_Note_Widget_C" null self))
      (`/Game/Blueprints/Placeables/interactions/wbp_Note_Widget.Initialise` _returnvalue (`self.Header`) (`self.Main Body Text`))
      (`UserWidget.AddToViewport` _returnvalue 0)
      (bind _asals_game_mode_sp (cast `/Game/AdvancedLocomotionV4/Blueprints/GameModes/ALS_GameMode_SP` (`GameplayStatics.GetGameMode`)))
      (set `/Game/AdvancedLocomotionV4/Blueprints/GameModes/ALS_GameMode_SP.Note` _returnvalue _asals_game_mode_sp))))

(fn `endhighlight`
  (if (> (`self.GetDistanceTo` (`GameplayStatics.GetPlayerCharacter` 0)) 400.0)
    (`self.Leave`)
    (`KismetSystemLibrary.K2_PauseTimerHandle` (`self.EndHighlightTimer`))))

(fn `UserConstructionScript`
  (switch `/Game/AdvancedLocomotionV4/Blueprints/CharacterLogic/InteractType` (`self.interactType`)
    (:`NewEnumerator1`
      (set `self.focused sprite` "/Game/Blueprints/Placeables/interactions/Textures/interact_Icon.interact_Icon"))
    (:`NewEnumerator2`
      (set `self.focused sprite` "/Game/Blueprints/Placeables/interactions/Textures/note.note"))))